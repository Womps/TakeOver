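; In-game PC code screen that checks a fixed four-digit code and reveals a letter-to-digit clue table when unlocked.
; Per-digit events append to the entry on a TextRender, capped by a counter, while printReturn clears both.
; printValid shows access granted in green with a sound, or access denied, then a timer reveals the table or clears the display.
; Raising the counter after success blocks digit entry; a random code generator sits unused.
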(event Custom|printValid
  (if (Utilities|Enum|Equal(Enum) (Variables|Default|Getcurrent) (Variables|Default|GetCODE_generation))
    (Rendering|Components|TextRender|SetText (Variables|Default|GetTextRender) (Utilities|Text|ToText(String) "Accès autorisé"))
    (Rendering|Components|TextRender|SetTextRenderColor (Variables|Default|GetTextRender) (Math|Color|MakeColor 0 255 0))
    (Audio|PlaySound2D "/Game/Sons/Deverouillage_ordi.Deverouillage_ordi" 2.0)
    (Variables|Default|Setcurrent "")
    (Variables|Default|Setcpt 4)
    (Utilities|Time|SetTimerbyEvent (delegate Custom|afficheInfo) (Math|Conversions|ToFloat(Integer) 3))
    (else
      (Rendering|Components|TextRender|SetText (Variables|Default|GetTextRender) (Utilities|Text|ToText(String) "Accès refusé"))
      (Variables|Default|Setcurrent "")
      (Variables|Default|Setcpt 0)
      (Utilities|Time|SetTimerbyEvent (delegate Custom|efface) (Math|Conversions|ToFloat(Integer) 1)))))

(event Custom|print1
  ;[1 1 1] Les chiffres
  (if (<= (Variables|Default|Getcpt) 3)
    (Rendering|Components|TextRender|SetText (Variables|Default|GetTextRender) (Utilities|Text|ToText(String) (Utilities|String|Append (Variables|Default|Getcurrent) (Utilities|String|MakeLiteralString "1"))))
    (Variables|Default|Setcurrent (Utilities|String|Append (Variables|Default|Getcurrent) (Utilities|String|MakeLiteralString "1")))
    (bind _result (Math|Integer|IncrementInt (Variables|Default|Getcpt))
      (:%20%20
        (Variables|Default|Setcpt _result)))))

(event Custom|print%202
  ;[1 1 1] Les chiffres
  (if (<= (Variables|Default|Getcpt) 3)
    (Rendering|Components|TextRender|SetText (Variables|Default|GetTextRender) (Utilities|Text|ToText(String) (Utilities|String|Append (Variables|Default|Getcurrent) (Utilities|String|MakeLiteralString "2"))))
    (Variables|Default|Setcurrent (Utilities|String|Append (Variables|Default|Getcurrent) (Utilities|String|MakeLiteralString "2")))
    (bind _result (Math|Integer|IncrementInt (Variables|Default|Getcpt))
      (:%20%20
        (Variables|Default|Setcpt _result)))))

(event Custom|print%203
  ;[1 1 1] Les chiffres
  (if (<= (Variables|Default|Getcpt) 3)
    (Rendering|Components|TextRender|SetText (Variables|Default|GetTextRender) (Utilities|Text|ToText(String) (Utilities|String|Append (Variables|Default|Getcurrent) (Utilities|String|MakeLiteralString "3"))))
    (Variables|Default|Setcurrent (Utilities|String|Append (Variables|Default|Getcurrent) (Utilities|String|MakeLiteralString "3")))
    (bind _result (Math|Integer|IncrementInt (Variables|Default|Getcpt))
      (:%20%20
        (Variables|Default|Setcpt _result)))))

(event Custom|print%204
  ;[1 1 1] Les chiffres
  (if (<= (Variables|Default|Getcpt) 3)
    (Rendering|Components|TextRender|SetText (Variables|Default|GetTextRender) (Utilities|Text|ToText(String) (Utilities|String|Append (Variables|Default|Getcurrent) (Utilities|String|MakeLiteralString "4"))))
    (Variables|Default|Setcurrent (Utilities|String|Append (Variables|Default|Getcurrent) (Utilities|String|MakeLiteralString "4")))
    (bind _result (Math|Integer|IncrementInt (Variables|Default|Getcpt))
      (:%20%20
        (Variables|Default|Setcpt _result)))))

(event Custom|print%205
  ;[1 1 1] Les chiffres
  (if (<= (Variables|Default|Getcpt) 3)
    (Rendering|Components|TextRender|SetText (Variables|Default|GetTextRender) (Utilities|Text|ToText(String) (Utilities|String|Append (Variables|Default|Getcurrent) (Utilities|String|MakeLiteralString "5"))))
    (Variables|Default|Setcurrent (Utilities|String|Append (Variables|Default|Getcurrent) (Utilities|String|MakeLiteralString "5")))
    (bind _result (Math|Integer|IncrementInt (Variables|Default|Getcpt))
      (:%20%20
        (Variables|Default|Setcpt _result)))))

(event Custom|print%206
  ;[1 1 1] Les chiffres
  (if (<= (Variables|Default|Getcpt) 3)
    (Rendering|Components|TextRender|SetText (Variables|Default|GetTextRender) (Utilities|Text|ToText(String) (Utilities|String|Append (Variables|Default|Getcurrent) (Utilities|String|MakeLiteralString "6"))))
    (Variables|Default|Setcurrent (Utilities|String|Append (Variables|Default|Getcurrent) (Utilities|String|MakeLiteralString "6")))
    (bind _result (Math|Integer|IncrementInt (Variables|Default|Getcpt))
      (:%20%20
        (Variables|Default|Setcpt _result)))))

(event Custom|print%207
  ;[1 1 1] Les chiffres
  (if (<= (Variables|Default|Getcpt) 3)
    (Rendering|Components|TextRender|SetText (Variables|Default|GetTextRender) (Utilities|Text|ToText(String) (Utilities|String|Append (Variables|Default|Getcurrent) (Utilities|String|MakeLiteralString "7"))))
    (Variables|Default|Setcurrent (Utilities|String|Append (Variables|Default|Getcurrent) (Utilities|String|MakeLiteralString "7")))
    (bind _result (Math|Integer|IncrementInt (Variables|Default|Getcpt))
      (:%20%20
        (Variables|Default|Setcpt _result)))))

(event Custom|print%208
  ;[1 1 1] Les chiffres
  (if (<= (Variables|Default|Getcpt) 3)
    (Rendering|Components|TextRender|SetText (Variables|Default|GetTextRender) (Utilities|Text|ToText(String) (Utilities|String|Append (Variables|Default|Getcurrent) (Utilities|String|MakeLiteralString "8"))))
    (Variables|Default|Setcurrent (Utilities|String|Append (Variables|Default|Getcurrent) (Utilities|String|MakeLiteralString "8")))
    (bind _result (Math|Integer|IncrementInt (Variables|Default|Getcpt))
      (:%20%20
        (Variables|Default|Setcpt _result)))))

(event Custom|print%209
  ;[1 1 1] Les chiffres
  (if (<= (Variables|Default|Getcpt) 3)
    (Rendering|Components|TextRender|SetText (Variables|Default|GetTextRender) (Utilities|Text|ToText(String) (Utilities|String|Append (Variables|Default|Getcurrent) (Utilities|String|MakeLiteralString "9"))))
    (Variables|Default|Setcurrent (Utilities|String|Append (Variables|Default|Getcurrent) (Utilities|String|MakeLiteralString "9")))
    (bind _result (Math|Integer|IncrementInt (Variables|Default|Getcpt))
      (:%20%20
        (Variables|Default|Setcpt _result)))))

(event Custom|print%200
  ;[1 1 1] Les chiffres
  (if (<= (Variables|Default|Getcpt) 3)
    (Rendering|Components|TextRender|SetText (Variables|Default|GetTextRender) (Utilities|Text|ToText(String) (Utilities|String|Append (Variables|Default|Getcurrent) (Utilities|String|MakeLiteralString "0"))))
    (Variables|Default|Setcurrent (Utilities|String|Append (Variables|Default|Getcurrent) (Utilities|String|MakeLiteralString "0")))
    (bind _result (Math|Integer|IncrementInt (Variables|Default|Getcpt))
      (:%20%20
        (Variables|Default|Setcpt _result)))))

(event Custom|printReturn
  (Rendering|Components|TextRender|SetText (Variables|Default|GetTextRender) (Utilities|Text|ToText(String) ""))
  (Variables|Default|Setcurrent "")
  (Variables|Default|Setcpt 0))

(event Custom|afficheInfo
  (bind _textrender (Variables|Default|GetTextRender))
  (Rendering|Components|TextRender|SetText _textrender (Utilities|Text|ToText(String) "a=3   b=5  c=7<br>d=1  e=2  f=9<br>g=4  h=8  i=6"))
  (Rendering|Components|TextRender|SetText (Variables|Default|Getligne%201) (Utilities|Text|ToText(String) ""))
  (Rendering|Components|TextRender|SetTextRenderColor _textrender (Math|Color|MakeColor 255 255 255))
  (Variables|Default|Setcpt 10)
  (Default|Log (Variables|Default|Getrefligne)))

(event Custom|efface
  (bind _textrender (Variables|Default|GetTextRender))
  (Rendering|Components|TextRender|SetText _textrender (Utilities|Text|ToText(String) ""))
  (Rendering|Components|TextRender|SetTextRenderColor _textrender (Math|Color|MakeColor 255 255 255)))

(event EventBeginPlay
  (Rendering|Components|TextRender|SetText (Variables|Default|GetTextRender) (Utilities|Text|ToText(String) ""))
  (Variables|Default|Setcurrent "")
  (Variables|Default|Setcpt 0)
  ;[1 1 1] Code fixe du PC
  (Variables|Default|SetCODE_generation "1953"))

(event EventTick
  (params (DeltaSeconds :type Float%20%28single-precision%29)))

(fn ConstructionScript)